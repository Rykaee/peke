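; Recycled diamond projectile that moves by a Speed offset each tick, scaled by truncated global time dilation rather than frame delta.
; On overlap it calls ApplyEffect, an empty stub here, if the other actor's name matches the player character.
; Any overlap then resets it to its initial X/Y at a random height, with a random scale that also sets its rounded Value.
; The respawn-trigger check's result is unused.
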(event `self.ReceiveTick`
  (params (DeltaSeconds :type "Float (single-precision)"))
  (`self.K2_AddActorWorldOffset` (* (`self.Speed`) (`KismetMathLibrary.FTrunc` (`GameplayStatics.GetGlobalTimeDilation`)))))

(event `self.ReceiveActorBeginOverlap`
  (params (OtherActor :type "Actor Object Reference"))
  (bind _returnvalue (`KismetSystemLibrary.GetObjectName` OtherActor))
  ;[1 1 1] Check if projectile hit Hero
  (bind _hitresult (`self.CheckHeroHit` _returnvalue))
  (if _hitresult
    (`self.ApplyEffect`)
    (else
      (`self.CheckRespawnHit` _returnvalue)))
  ;[1 1 1] Reset projectile values
  (`self.ResetPosition`)
  (`self.ResetScaleAndValue`))

(fn `ApplyEffect`)

(fn `CheckHeroHit`
  (params (OtherObjectName :type String))
  (returns (HitResult :type Boolean))
  (return (`KismetStringLibrary.EqualEqual_StrStr` OtherObjectName (`KismetSystemLibrary.GetObjectName` (`GameplayStatics.GetPlayerCharacter` 0)))))

(fn `CheckRespawnHit`
  (params (OtherObjectName :type String))
  (returns (HitResult :type Boolean))
  (return (`KismetStringLibrary.EqualEqual_StrStr` OtherObjectName (`self.RespawnTriggerName`))))

(fn `ResetPosition`
  (`self.K2_SetActorLocation` (`KismetMathLibrary.MakeVector` (.x (`self.InitialPosition`)) (.y (`self.InitialPosition`)) (`KismetMathLibrary.RandomFloatInRange` 300.0 400.0))))

(fn `ResetScaleAndValue`
  (bind _output_get (set `self.Scale` (`KismetMathLibrary.RandomFloatInRange` 1.0 5.0)))
  (bind _returnvalue (/ _output_get 10.0))
  (`self.SetActorScale3D` (`KismetMathLibrary.MakeVector` _returnvalue _returnvalue _returnvalue))
  (set `self.Value` (`KismetMathLibrary.Round` (`self.Scale`))))

(fn `UserConstructionScript`)