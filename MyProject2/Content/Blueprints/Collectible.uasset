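; Collectible actor that scrolls by a Speed offset every tick, scaled by truncated global time dilation rather than delta time.
; Reset functions return it to its initial X/Y at a random height and randomize its uniform scale, with Value rounded from that scale.
; Name-comparison helpers identify hits with the player character or respawn trigger, but nothing in this Blueprint calls them or the resets.
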(event `self.ReceiveTick`
  (params (DeltaSeconds :type "Float (single-precision)"))
  (`self.K2_AddActorWorldOffset` (* (`self.Speed`) (`KismetMathLibrary.FTrunc` (`GameplayStatics.GetGlobalTimeDilation`)))))

(fn `CheckHeroHit`
  (params (OtherObjectName :type String))
  (returns (HitResult :type Boolean))
  (return (`KismetStringLibrary.EqualEqual_StrStr` OtherObjectName (`KismetSystemLibrary.GetObjectName` (`GameplayStatics.GetPlayerCharacter` 0)))))

(fn `CheckRespawnHit`
  (params (OtherObjectName :type String))
  (returns (HitResult :type Boolean))
  (return (`KismetStringLibrary.EqualEqual_StrStr` OtherObjectName (`self.RespawnTriggerName`))))

(fn `ResetPosition`
  (`self.K2_SetActorLocation` (`KismetMathLibrary.MakeVector` (.x (`self.InitialPosition`)) (.y (`self.InitialPosition`)) (`KismetMathLibrary.RandomFloatInRange` 100.0 200.0))))

(fn `ResetScaleAndValue`
  (bind _output_get (set `self.Scale` (`KismetMathLibrary.RandomFloatInRange` 1.0 5.0)))
  (`self.SetActorScale3D` (`KismetMathLibrary.MakeVector` _output_get _output_get _output_get))
  (set `self.Value` (`KismetMathLibrary.Round` (`self.Scale`))))

(fn `UserConstructionScript`)