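; Timu is a diamond collectible that reports its Value through the TimuCollectedED event dispatcher when the Hero collects it.
; On overlap, it checks the other actor's object name for a Hero hit, otherwise runs a respawn-hit check, then resets its position, scale and value either way.
; It builds on a parent class for Tick and ApplyEffect, with its ApplyEffect override also firing the collected dispatcher.
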(event `self.ReceiveActorBeginOverlap`
  (params (OtherActor :type "Actor Object Reference"))
  (bind _returnvalue (`KismetSystemLibrary.GetObjectName` OtherActor))
  ;[1 1 1] Check if diamond hit Hero
  (bind _hitresult (`self.CheckHeroHit` _returnvalue))
  (if _hitresult
    ;[1 1 1] Send message that diamond was collected by Hero
    (`self.TimuCollected_ED` (`self.Value`))
    (else
      (`self.CheckRespawnHit` _returnvalue)))
  ;[1 1 1] Reset Diamond position
  (`self.ResetPosition`)
  (`self.ResetScaleAndValue`))

(event `self.ReceiveTick`
  (params (DeltaSeconds :type "Float (single-precision)"))
  (`parent.ReceiveTick` 0.0))

(fn `ApplyEffect`
  (`parent.ApplyEffect`)
  (`self.TimuCollected_ED` (`self.Value`)))

(fn `UserConstructionScript`)