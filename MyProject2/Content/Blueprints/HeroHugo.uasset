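; HeroHugo is a player-controlled side-scrolling character with a flipbook sprite that moves along the Y axis and jumps.
; Two input axes feed movement in opposite directions, and BeginPlay sets game-only input.
; Pressing Jump switches to the jump flipbook (Hyppy1), and a capsule hit on an actor tagged "Surface" restores the run flipbook (Juoksu), each with its own play rate.
; StopJumping is present but unconnected.
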(event `self.CapsuleComponent.OnComponentHit`
  (params (HitComponent :type "PrimitiveComponent Object Reference") (OtherActor :type "Actor Object Reference") (OtherComp :type "PrimitiveComponent Object Reference") (NormalImpulse :type "Vector Structure") (Hit :type "HitResult Structure (by ref)"))
  (if (`self.ActorHasTag` OtherActor "Surface")
    (`PaperFlipbookComponent.SetFlipbook` (`self.Sprite`) "/Game/Flipbooks/juoksu.juoksu")
    (`PaperFlipbookComponent.SetPlayRate` (`self.Sprite`) 0.5)))

(event `InputAction|Jump`
  (params (Key :type "Key Structure"))
  (:`Pressed`
    (`PaperFlipbookComponent.SetFlipbook` (`self.Sprite`) "/Game/Flipbooks/hyppy1.hyppy1")
    (`self.Jump`)
    (`PaperFlipbookComponent.SetPlayRate` (`self.Sprite`) 0.1)))

(event `self.ReceiveBeginPlay`
  (`WidgetBlueprintLibrary.SetInputMode_GameOnly` (`GameplayStatics.GetPlayerController` 0)))

(event `InputAxis|Move_right`
  (params (AxisValue :type "Float (single-precision)"))
  (`self.AddMovementInput` (0.0 -1.0 0.0) AxisValue))

(event `InputAxis|Move_left`
  (params (AxisValue :type "Float (single-precision)"))
  (`self.AddMovementInput` (0.0 1.0 0.0) AxisValue))

(fn `UserConstructionScript`)